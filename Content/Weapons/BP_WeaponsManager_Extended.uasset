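; Weapons manager component that gives a Character its starting weapons and handles equipping and unequipping them.
; Given weapons spawn attached to stowed sockets; equipping looks one up by class, and requesting the held class again unequips it.
; Each switch applies the weapon's or unarmed config's anim class and movement settings.
; Montage notifies or interruption trigger socket reattachment, with unarmed movement restored at that point too.
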(event `self.ReceiveBeginPlay`
  (bind _ascharacter (cast `Character` (`self.GetOwner`)))
  (set `self.OwningCharacterRef` _ascharacter)
  (for _array_element (`self.StartingWeapons`)
    (`self.GiveWeapons` _array_element)))

(event `GiveWeapons`
  (params (WeaponClass :type "/Game/Weapons/BP_WeaponBase Class Reference"))
  (bind _returnvalue (`|SpawnActorFromClass` WeaponClass (`KismetMathLibrary.MakeTransform` (0.0 0.0 0.0)) "Undefined" "MultiplyWithRoot" null null))
  (`KismetArrayLibrary.Array_AddUnique` (`self.StowedWeapons`) _returnvalue)
  (`Actor.K2_AttachToComponent` _returnvalue (`Character.Mesh` (`self.OwningCharacterRef`)) (`.StowedSocket_17_434573874544E6CDCF3E2D862BA5FF85` (break `/Game/Weapons/Data/S_WeaponConfig` (`/Game/Weapons/BP_WeaponBase.WeaponConfig` _returnvalue))) "SnapToTarget" "SnapToTarget" "SnapToTarget" true))

(event `EquipWeapon`
  (params (WeaponClass :type "/Game/Weapons/BP_WeaponBase Class Reference"))
  (bind _equippedweapon (`self.EquippedWeapon`))
  (bind _charactermovement (`Character.CharacterMovement` (`self.OwningCharacterRef`)))
  (bind _mesh (`Character.Mesh` (`self.OwningCharacterRef`)))
  (bind (_abilitiestogrant _animclass _equipmontage _equippedsocket) (break `/Game/Weapons/Data/S_WeaponConfig` (`/Game/Weapons/BP_WeaponBase.WeaponConfig` _equippedweapon)))
  (`self.OwningCharacterRef`
    (:`then`
      (bind _equippedweapon_2 (`self.EquippedWeapon`)
        (:`then`
          (if (== (`GameplayStatics.GetObjectClass` _equippedweapon_2) WeaponClass)
            (`self.UnequipWeapon`)
            (else
              (`self.UnequipWeapon`)
              (bind _stowedweapon (`self.GetStowedWeaponByClass` WeaponClass :!label _label))
              (`/Engine/EditorBlueprintResources/StandardMacros.IsValid` _stowedweapon
                (:`Is Valid`
                  (bind _output_get (set `self.EquippedWeapon` _stowedweapon))
                  (bind ((`AnimClass_10_094C8F16420642C7CC31FB9957B13DAB` _animclass_2) (`EquipMontage_23_5A4D3B3445B9F3165CE6E58847601DEF` _equipmontage_2) (`EquippedSocket_7_EF01717E44D93EE6306D10ACBDF0F421` _equippedsocket_2) (`UnequipMontage_24_DCCDB4F44B6AE40A98620D9F6187567B` _unequipmontage) (`StowedSocket_17_434573874544E6CDCF3E2D862BA5FF85` _stowedsocket) (`MovementProperties_14_3F91ABEA4C31901BB815E18893C2E7D6` _movementproperties)) (break `/Game/Weapons/Data/S_WeaponConfig` (`/Game/Weapons/BP_WeaponBase.WeaponConfig` _output_get)))
                  (`SkeletalMeshComponent.SetAnimInstanceClass` (`Character.Mesh` (`self.OwningCharacterRef`)) _animclass_2)
                  (bind (_maxwalkspeed _orientrotationtomovement _usecontrollerdesierdrotation) (break `/Game/Weapons/Data/S_MovementProperties` _movementproperties))
                  (set `CharacterMovementComponent.MaxWalkSpeed` _maxwalkspeed _charactermovement)
                  (set `CharacterMovementComponent.bOrientRotationToMovement` _orientrotationtomovement _charactermovement)
                  (set `CharacterMovementComponent.bUseControllerDesiredRotation` _usecontrollerdesierdrotation _charactermovement)
                  (bind _notifyname (`|PlayMontage` _mesh _equipmontage 1.0 0.0 "None" false)
                    (:`OnInterrupted`
                      _)
                    (:`OnNotifyBegin`
                      (switch `name` _notifyname
                        (:`Equip`
                          _))))
                  (`Actor.K2_AttachToComponent` _equippedweapon _mesh _equippedsocket "SnapToTarget" "SnapToTarget" "SnapToTarget" true))))))
        (:`else`
          (goto _label))))
    (:`else`)))

(event `UnequipWeapon`
  (bind _previouslyequippedweapon (`self.PreviouslyEquippedWeapon`))
  (bind _charactermovement (`Character.CharacterMovement` (`self.OwningCharacterRef`)))
  (bind _mesh (`Character.Mesh` (`self.OwningCharacterRef`)))
  (bind (_maxwalkspeed _orientrotationtomovement _usecontrollerdesierdrotation) (break `/Game/Weapons/Data/S_MovementProperties` (`.MovementProperties_14_3F91ABEA4C31901BB815E18893C2E7D6` (break `/Game/Weapons/Data/S_WeaponConfig` (`self.UnarmedWeaponConfig`)))))
  (bind _equippedweapon (`self.EquippedWeapon`)
    (:`then`
      (set `self.PreviouslyEquippedWeapon` _equippedweapon)
      (set `self.EquippedWeapon` null)
      (`SkeletalMeshComponent.SetAnimInstanceClass` _mesh (`.AnimClass_10_094C8F16420642C7CC31FB9957B13DAB` (break `/Game/Weapons/Data/S_WeaponConfig` (`self.UnarmedWeaponConfig`))))
      (bind _notifyname (`|PlayMontage` _mesh (`.UnequipMontage_24_DCCDB4F44B6AE40A98620D9F6187567B` (break `/Game/Weapons/Data/S_WeaponConfig` (`/Game/Weapons/BP_WeaponBase.WeaponConfig` (`self.PreviouslyEquippedWeapon`)))) 1.0 0.0 "None" false)
        (:`OnInterrupted`
          _)
        (:`OnNotifyBegin`
          (switch `name` _notifyname
            (:`UnEquip`
              _))))
      (`Actor.K2_AttachToComponent` _previouslyequippedweapon _mesh (`.StowedSocket_17_434573874544E6CDCF3E2D862BA5FF85` (break `/Game/Weapons/Data/S_WeaponConfig` (`/Game/Weapons/BP_WeaponBase.WeaponConfig` _previouslyequippedweapon))) "SnapToTarget" "SnapToTarget" "SnapToTarget" true)
      (set `CharacterMovementComponent.MaxWalkSpeed` _maxwalkspeed _charactermovement)
      (set `CharacterMovementComponent.bOrientRotationToMovement` _orientrotationtomovement _charactermovement)
      (set `CharacterMovementComponent.bUseControllerDesiredRotation` _usecontrollerdesierdrotation _charactermovement))
    (:`else`)))

(fn `GetStowedWeaponByClass`
  (params (WeaponClass :type "/Game/Weapons/BP_WeaponBase Class Reference"))
  (returns (StowedWeapon :type "/Game/Weapons/BP_WeaponBase Object Reference"))
  (for _array_element (`self.StowedWeapons`)
    (if (== (`GameplayStatics.GetObjectClass` _array_element) WeaponClass)
      (return _array_element))))