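; Weapons manager component for Nexus_BaseCharacter that spawns starting weapons on the server, stows them on mesh sockets and handles equip and unequip.
; Equipping by class toggles or swaps weapons, granting and removing their GAS abilities.
; Each weapon's config, or an unarmed fallback, drives anim class and movement settings.
; Montage notifies or interruptions time socket attachment, and OnRep_EquippedWeapon reapplies the presentation on clients.
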(event `self.ReceiveBeginPlay`
  (bind _asnexus_base_character (cast `Nexus_BaseCharacter` (`self.GetOwner`)))
  (set `self.OwningCharacterRef` _asnexus_base_character)
  (`/Engine/EditorBlueprintResources/ActorComponentMacros.Switch Has Authority`
    (:`Authority`
      (for _array_element (`self.StartingWeapons`)
        (`self.GiveWeapons` _array_element)))))

(event `GiveWeapons`
  (params (WeaponClass :type "/Game/_GameplayAbilitySystem/Weapons/BP_WeaponBase Class Reference"))
  (bind _returnvalue (`|SpawnActorFromClass` WeaponClass (`KismetMathLibrary.MakeTransform` (0.0 0.0 0.0)) "Undefined" "MultiplyWithRoot" null (`self.OwningCharacterRef`)))
  (`KismetArrayLibrary.Array_AddUnique` (`self.StowedWeapons`) _returnvalue)
  (`Actor.K2_AttachToComponent` _returnvalue (`Character.Mesh` (`self.OwningCharacterRef`)) (`.StowedSocket_17_434573874544E6CDCF3E2D862BA5FF85` (break `/Game/_GameplayAbilitySystem/Weapons/Data/S_WeaponConfig` (`/Game/_GameplayAbilitySystem/Weapons/BP_WeaponBase.WeaponConfig` _returnvalue))) "SnapToTarget" "SnapToTarget" "SnapToTarget" true))

(event `EquipWeapon`
  (params (WeaponClass :type "/Game/_GameplayAbilitySystem/Weapons/BP_WeaponBase Class Reference"))
  ;[0.007246 0 0.125] Equip Weapon
  (`/Engine/EditorBlueprintResources/ActorComponentMacros.Switch Has Authority`
    (:`Authority`
      (`self.OwningCharacterRef`
        (:`then`
          (bind _equippedweapon (`self.EquippedWeapon`)
            (:`then`
              (if (== (`GameplayStatics.GetObjectClass` _equippedweapon) WeaponClass)
                (`self.UnequipWeapon`)
                (else
                  (`self.UnequipWeapon`)
                  (bind _stowedweapon (`self.GetStowedWeaponByClass` WeaponClass :!label _label))
                  (`/Engine/EditorBlueprintResources/StandardMacros.IsValid` _stowedweapon
                    (:`Is Valid`
                      (set `self.EquippedWeapon` _stowedweapon)
                      (bind _returnvalue (`Nexus_BaseCharacter.GrantAbilities` (`self.OwningCharacterRef`) (`.AbilitiesToGrant_3_11D03FBD425EEE2F38634B86F5B0AEBA` (break `/Game/_GameplayAbilitySystem/Weapons/Data/S_WeaponConfig` (`/Game/_GameplayAbilitySystem/Weapons/BP_WeaponBase.WeaponConfig` (`self.EquippedWeapon`))))))
                      (set `self.AbilitiesGrantedByWeapon` _returnvalue)
                      (`self.SetEquippepWeaponProperties`))))))
            (:`else`
              (goto _label))))
        (:`else`)))))

(event `SetEquippepWeaponProperties`
  (bind _equippedweapon (`self.EquippedWeapon`))
  (bind _charactermovement (`Character.CharacterMovement` (`self.OwningCharacterRef`)))
  (bind _mesh (`Character.Mesh` (`self.OwningCharacterRef`)))
  (bind ((`EquipMontage_23_5A4D3B3445B9F3165CE6E58847601DEF` _equipmontage) (`EquippedSocket_7_EF01717E44D93EE6306D10ACBDF0F421` _equippedsocket)) (break `/Game/_GameplayAbilitySystem/Weapons/Data/S_WeaponConfig` (`/Game/_GameplayAbilitySystem/Weapons/BP_WeaponBase.WeaponConfig` _equippedweapon)))
  ;[0.25 0 0.2218] Set Equipped Weapon Properties
  (bind _equippedweapon_2 (`self.EquippedWeapon`)
    (:`then`
      (bind ((`AnimClass_10_094C8F16420642C7CC31FB9957B13DAB` _animclass) (`MovementProperties_14_3F91ABEA4C31901BB815E18893C2E7D6` _movementproperties)) (break `/Game/_GameplayAbilitySystem/Weapons/Data/S_WeaponConfig` (`/Game/_GameplayAbilitySystem/Weapons/BP_WeaponBase.WeaponConfig` _equippedweapon_2)))
      (`SkeletalMeshComponent.SetAnimInstanceClass` (`Character.Mesh` (`self.OwningCharacterRef`)) _animclass)
      (bind (_maxwalkspeed _orientrotationtomovement _usecontrollerdesierdrotation) (break `/Game/_GameplayAbilitySystem/Weapons/Data/S_MovementProperties` _movementproperties))
      (set `CharacterMovementComponent.MaxWalkSpeed` _maxwalkspeed _charactermovement)
      (set `CharacterMovementComponent.bOrientRotationToMovement` _orientrotationtomovement _charactermovement)
      (set `CharacterMovementComponent.bUseControllerDesiredRotation` _usecontrollerdesierdrotation _charactermovement)
      (bind _notifyname (`|PlayMontage` _mesh _equipmontage 1.0 0.0 "None" false)
        (:`then`
          (`self.OnWeaponChanged` (`self.EquippedWeapon`)))
        (:`OnInterrupted`
          (`Actor.K2_AttachToComponent` _equippedweapon _mesh _equippedsocket "SnapToTarget" "SnapToTarget" "SnapToTarget" true :!label _label_2))
        (:`OnNotifyBegin`
          (switch `name` _notifyname
            (:`Equip`
              (goto _label_2))))))
    (:`else`)))

(event `UnequipWeapon`
  ;[0.007246 0 0.125] UnEquip Weapon
  (bind _equippedweapon (`self.EquippedWeapon`)
    (:`then`
      (set `self.PreviouslyEquippedWeapon` _equippedweapon)
      (set `self.EquippedWeapon` null)
      (`Nexus_BaseCharacter.RemoveAbilities` (`self.OwningCharacterRef`) (`self.AbilitiesGrantedByWeapon`))
      (`self.SetUnarmedWeaponProperties`))
    (:`else`)))

(event `SetUnarmedWeaponProperties`
  (bind _previouslyequippedweapon (`self.PreviouslyEquippedWeapon`))
  (bind _charactermovement (`Character.CharacterMovement` (`self.OwningCharacterRef`)))
  (bind _mesh (`Character.Mesh` (`self.OwningCharacterRef`)))
  (bind (_maxwalkspeed _orientrotationtomovement _usecontrollerdesierdrotation) (break `/Game/_GameplayAbilitySystem/Weapons/Data/S_MovementProperties` (`.MovementProperties_14_3F91ABEA4C31901BB815E18893C2E7D6` (break `/Game/_GameplayAbilitySystem/Weapons/Data/S_WeaponConfig` (`self.UnarmedWeaponConfig`)))))
  (`SkeletalMeshComponent.SetAnimInstanceClass` _mesh (`.AnimClass_10_094C8F16420642C7CC31FB9957B13DAB` (break `/Game/_GameplayAbilitySystem/Weapons/Data/S_WeaponConfig` (`self.UnarmedWeaponConfig`))))
  (bind _notifyname (`|PlayMontage` _mesh (`.UnequipMontage_24_DCCDB4F44B6AE40A98620D9F6187567B` (break `/Game/_GameplayAbilitySystem/Weapons/Data/S_WeaponConfig` (`/Game/_GameplayAbilitySystem/Weapons/BP_WeaponBase.WeaponConfig` (`self.PreviouslyEquippedWeapon`)))) 1.0 0.0 "None" false)
    (:`OnInterrupted`
      _)
    (:`OnNotifyBegin`
      (switch `name` _notifyname
        (:`UnEquip`
          _))))
  (`Actor.K2_AttachToComponent` _previouslyequippedweapon _mesh (`.StowedSocket_17_434573874544E6CDCF3E2D862BA5FF85` (break `/Game/_GameplayAbilitySystem/Weapons/Data/S_WeaponConfig` (`/Game/_GameplayAbilitySystem/Weapons/BP_WeaponBase.WeaponConfig` _previouslyequippedweapon))) "SnapToTarget" "SnapToTarget" "SnapToTarget" true)
  (set `CharacterMovementComponent.MaxWalkSpeed` _maxwalkspeed _charactermovement)
  (set `CharacterMovementComponent.bOrientRotationToMovement` _orientrotationtomovement _charactermovement)
  (set `CharacterMovementComponent.bUseControllerDesiredRotation` _usecontrollerdesierdrotation _charactermovement)
  (`self.OnWeaponChanged` null))

(fn `GetStowedWeaponByClass`
  (params (WeaponClass :type "/Game/_GameplayAbilitySystem/Weapons/BP_WeaponBase Class Reference"))
  (returns (StowedWeapon :type "/Game/_GameplayAbilitySystem/Weapons/BP_WeaponBase Object Reference"))
  (for _array_element (`self.StowedWeapons`)
    (if (== (`GameplayStatics.GetObjectClass` _array_element) WeaponClass)
      (return _array_element))))

(fn `OnRep_EquippedWeapon`
  (`self.EquippedWeapon`
    (:`then`
      (`self.SetEquippepWeaponProperties`))
    (:`else`
      (`self.SetUnarmedWeaponProperties`))))