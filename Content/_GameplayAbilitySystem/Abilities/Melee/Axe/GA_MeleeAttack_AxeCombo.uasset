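; Melee axe combo gameplay ability that extends a parent attack ability and scales hit damage with the current combo count.
; When the montage starts, gameplay event listeners open and close a combo input window.
; Input received inside the window lets the combo continue and increments the count when the window closes; otherwise the ability ends.
; Owners without a player controller always continue the combo, bypassing the input check.
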(event `self.K2_ActivateAbility`
  (`parent.K2_ActivateAbility`)
  (set `self.AlwaysContinueCombo` (not (`self.HasPC`))))

(event `self.MontageStarted`
  (set `self.ComboCount` 1)
  (`AbilityTask_WaitGameplayEvent.WaitGameplayEvent` (struct :`TagName` "_Nexus.Events.Combo.Start") null
    (:`then`
      (`AbilityTask_WaitGameplayEvent.WaitGameplayEvent` (struct :`TagName` "_Nexus.Events.Combo.End") null
        (:`then`
          (`AbilityTask_WaitGameplayEvent.WaitGameplayEvent` (struct :`TagName` "_Nexus.Events.Combo.Input") null
            (:`EventReceived`
              (set `self.RecievedInputAtRightTime` (`self.IsWithinComboWindow`)))))
        (:`EventReceived`
          (set `self.IsWithinComboWindow` false)
          (if (or (`self.RecievedInputAtRightTime`) (`self.AlwaysContinueCombo`))
            (`/Engine/EditorBlueprintResources/StandardMacros.IncrementInt` (`self.ComboCount`))
            (else
              (`self.K2_EndAbility`))))))
    (:`EventReceived`
      (set `self.IsWithinComboWindow` true)
      (set `self.RecievedInputAtRightTime` false))))

(event `self.HandlehitScanBegin`
  (set `self.DamageMagnitude` (* -34.0 (`self.ComboCount`)))
  (`parent.HandlehitScanBegin`))