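; Base melee attack gameplay ability that plays an attack montage using the avatar's equipped weapon, ending immediately if none exists.
; On the server, gameplay events from the montage window open and close the weapon's hit scan.
; Hit scan start passes a damage effect spec with a set-by-caller magnitude to the weapon.
; Hit scanning is also stopped when the ability ends, and MontageStarted is an empty hook.
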(event `self.K2_ActivateAbility`
  (bind _returnvalue (`Actor.GetComponentByClass` (`self.GetAvatarActorFromActorInfo`) "/Game/_GameplayAbilitySystem/Weapons/BP_WeaponsManager_Extended.BP_WeaponsManager_Extended_C"))
  (`/Engine/EditorBlueprintResources/StandardMacros.IsValid` _returnvalue
    (:`Is Valid`
      (bind _equippedweapon (`/Game/_GameplayAbilitySystem/Weapons/BP_WeaponsManager_Extended.EquippedWeapon` _returnvalue)
        (:`then`
          (set `self.EquippedWeapon` _equippedweapon)
          (`AbilityTask_PlayMontageAndWait.CreatePlayMontageAndWaitProxy` "None" (`self.AttackMontage`) 1.0 "None" true 1.0 0.0 true
            (:`then`
              (`self.MontageStarted`)
              (`self.K2_HasAuthority`
                (:`True`
                  (`AbilityTask_WaitGameplayEvent.WaitGameplayEvent` (struct :`TagName` "_Nexus.Events.HitScan.Begin") null
                    (:`then`
                      (`AbilityTask_WaitGameplayEvent.WaitGameplayEvent` (struct :`TagName` "_Nexus.Events.HitScan.End") null
                        (:`EventReceived`
                          (`self.HandleHitScanEnd`))))
                    (:`EventReceived`
                      (`self.HandlehitScanBegin`))))))
            (:`OnCompleted`
              (`self.K2_EndAbility` :!label _label))
            (:`OnInterrupted`
              (goto _label))
            (:`OnCancelled`
              (goto _label))))
        (:`else`
          (`self.K2_EndAbility` :!label _label_2))))
    (:`Is Not Valid`
      (goto _label_2))))

(event `HandlehitScanBegin`
  (bind _equippedweapon (`self.EquippedWeapon`)
    (:`then`
      (bind _returnvalue (`AbilitySystemBlueprintLibrary.AssignTagSetByCallerMagnitude` (`self.MakeOutgoingGameplayEffectSpec` (`self.DamageEffectClass`)) (struct :`TagName` "_Nexus.Data.Damage") (`self.DamageMagnitude`)))
      (`/Game/_GameplayAbilitySystem/Weapons/BP_WeaponBase.HitScanStart` _equippedweapon _returnvalue))
    (:`else`)))

(event `HandleHitScanEnd`
  (bind _equippedweapon (`self.EquippedWeapon`)
    (:`then`
      (`/Game/_GameplayAbilitySystem/Weapons/BP_WeaponBase.HitScanEnd` _equippedweapon))
    (:`else`)))

(event `MontageStarted`)

(event `self.K2_OnEndAbility`
  (params (bWasCancelled :type Boolean))
  (`self.HandleHitScanEnd`))