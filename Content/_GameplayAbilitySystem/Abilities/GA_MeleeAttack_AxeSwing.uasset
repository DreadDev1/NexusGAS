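; GA_MeleeAttack_AxeSwing is a gameplay ability that performs an axe swing melee attack with the avatar's equipped weapon.
; It fetches the weapon from the weapons manager component, ending if none exists, and plays the swing montage.
; On authority, gameplay events open and close the weapon's hit scan, passing an instant damage spec with a set-by-caller magnitude.
; Ending the ability also stops the hit scan.
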(event `self.K2_ActivateAbility`
  (bind _returnvalue (`Actor.GetComponentByClass` (`self.GetAvatarActorFromActorInfo`) "/Game/_GameplayAbilitySystem/Weapons/BP_WeaponsManager_Extended.BP_WeaponsManager_Extended_C"))
  (`/Engine/EditorBlueprintResources/StandardMacros.IsValid` _returnvalue
    (:`Is Valid`
      (bind _equippedweapon (`/Game/_GameplayAbilitySystem/Weapons/BP_WeaponsManager_Extended.EquippedWeapon` _returnvalue)
        (:`then`
          (set `self.EquippedWeapon` _equippedweapon)
          (`AbilityTask_PlayMontageAndWait.CreatePlayMontageAndWaitProxy` "None" "/Game/_GameplayAbilitySystem/Characters/Mannequins/Anims/Axe/Montage_MeleeAttack_AxeSwing.Montage_MeleeAttack_AxeSwing" 1.0 "None" true 1.0 0.0 true
            (:`then`
              (`self.K2_HasAuthority`
                (:`True`
                  (`AbilityTask_WaitGameplayEvent.WaitGameplayEvent` (struct :`TagName` "_Nexus.Events.HitScan.Begin") null
                    (:`then`
                      (`AbilityTask_WaitGameplayEvent.WaitGameplayEvent` (struct :`TagName` "_Nexus.Events.HitScan.End") null
                        (:`EventReceived`
                          (`/Game/_GameplayAbilitySystem/Weapons/BP_WeaponBase.HitScanEnd` (stale _equippedweapon_2)))))
                    (:`EventReceived`
                      (bind _equippedweapon_2 (`self.EquippedWeapon`)
                        (:`then`
                          (bind _returnvalue_2 (`AbilitySystemBlueprintLibrary.AssignTagSetByCallerMagnitude` (`self.MakeOutgoingGameplayEffectSpec` "/Game/_GameplayAbilitySystem/Effects/GE_DamageInstant.GE_DamageInstant_C") (struct :`TagName` "_Nexus.Data.Damage") -34.0))
                          (`/Game/_GameplayAbilitySystem/Weapons/BP_WeaponBase.HitScanStart` _equippedweapon_2 _returnvalue_2))
                        (:`else`)))))))
            (:`OnCompleted`
              (`self.K2_EndAbility` :!label _label))
            (:`OnInterrupted`
              (goto _label))
            (:`OnCancelled`
              (goto _label))))
        (:`else`
          (`self.K2_EndAbility` :!label _label_2))))
    (:`Is Not Valid`
      (goto _label_2))))

(event `self.K2_OnEndAbility`
  (params (bWasCancelled :type Boolean))
  (bind _equippedweapon (`self.EquippedWeapon`)
    (:`then`
      (`/Game/_GameplayAbilitySystem/Weapons/BP_WeaponBase.HitScanEnd` _equippedweapon))
    (:`else`)))