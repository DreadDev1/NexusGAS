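; GA_Dash is a gameplay ability that dashes the avatar with a root motion constant force.
; The direction comes from the event target data's hit Location, falling back to the actor's forward vector when that is zero.
; Cost is committed on activation and cooldown on end, with a Dash gameplay cue active in between.
; When the force finishes, velocity is clamped to the pawn's max movement speed and the ability ends.
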(event `self.K2_ActivateAbilityFromEvent`
  (params (EventData :type "GameplayEventData Structure (by ref)"))
  (bind (_bblockinghit _binitialoverlap _time _distance _location) (`GameplayStatics.BreakHitResult` (`AbilitySystemBlueprintLibrary.GetHitResultFromTargetData` (`.TargetData` (break `GameplayEventData` EventData)))))
  (`self.K2_CommitAbilityCost` false)
  (`AbilityTask_ApplyRootMotionConstantForce.ApplyRootMotionConstantForce` "None" (`KismetMathLibrary.SelectVector` (`Actor.GetActorForwardVector` (`self.GetAvatarActorFromActorInfo`)) _location (== _location (0.0 0.0 0.0))) 2000.0 0.5 false null "ClampVelocity" (0.0 0.0 0.0) (`self.GetMaxSpeed`)
    (:`then`
      (`self.K2_AddGameplayCue` (struct :`TagName` "GameplayCue._Nexus.Dash.Active")))
    (:`OnFinish`
      (`self.K2_EndAbility`))))

(event `self.K2_OnEndAbility`
  (params (bWasCancelled :type Boolean))
  (`self.K2_CommitAbilityCooldown` false))

(fn `GetMaxSpeed`
  (returns (MaxSpeed :type "Float (double-precision)"))
  (bind _aspawn (cast `Pawn` (`self.GetAvatarActorFromActorInfo`))
    (:`then`
      (return (`MovementComponent.GetMaxSpeed` (`Pawn.GetMovementComponent` _aspawn))))
    (:`CastFailed`
      (return 50.0))))