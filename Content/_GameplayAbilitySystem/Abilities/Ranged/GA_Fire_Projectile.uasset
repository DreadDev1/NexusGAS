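; Gameplay ability for ranged attacks that plays a fire montage and launches a projectile when the montage's FireProjectile gameplay event arrives.
; It aims at the avatar's attack target, falling back to an instant line trace if HasPC, otherwise ending.
; The projectile spawns on authority from the equipped weapon's spawn point or actor location, carrying a SetByCaller damage effect spec.
; The ability also ends when the montage finishes or is interrupted.
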(event `self.K2_ActivateAbility`
  (`AbilityTask_PlayMontageAndWait.CreatePlayMontageAndWaitProxy` "None" (`self.AnimationMontage`)
    (:`then`
      (`AbilityTask_WaitGameplayEvent.WaitGameplayEvent` (struct :`TagName` "_Nexus.Events.Weapon.FireProjectile") null
        (:`EventReceived`
          (bind _attacktarget (message `/Game/_GameplayAbilitySystem/Interface/BPI_Targeting.GetAttackTarget` (`self.GetAvatarActorFromActorInfo`)))
          (`/Engine/EditorBlueprintResources/StandardMacros.IsValid` _attacktarget
            (:`Is Valid`
              (`self.ShootProjectile` (`Actor.K2_GetActorLocation` _attacktarget)))
            (:`Is Not Valid`
              (if (`self.HasPC`)
                (bind (_asynctaskproxy _data) (`AbilityTask_WaitTargetData.WaitTargetData` "None" "Instant" "/Script/GameplayAbilities.GameplayAbilityTargetActor_SingleLineTrace" 999999.0 (struct :`Name` "NoCollision") true (`self.MakeTargetLocationInfoFromOwnerActor`) (struct) null (struct) true)
                  (:`ValidData`
                    (`self.ShootProjectile` (`AbilitySystemBlueprintLibrary.GetTargetDataEndPoint` _data))))
                (else
                  (`self.K2_EndAbility`))))))))
    (:`OnCompleted`
      (`self.K2_EndAbility` :!label _label))
    (:`OnBlendOut`
      (goto _label))
    (:`OnInterrupted`
      (goto _label))
    (:`OnCancelled`
      (goto _label))))

(event `ShootProjectile`
  (params (TargetLocation :type "Vector Structure"))
  (bind _returnvalue (`AbilitySystemBlueprintLibrary.AssignTagSetByCallerMagnitude` (`self.MakeOutgoingGameplayEffectSpec` (`self.DamageEffectClass`)) (struct :`TagName` "_Nexus.Data.Damage") (`self.DamageMagnitude`)))
  (bind _location (`self.GetSpawnLocation`))
  (`GameplayTask_SpawnActor.SpawnActor` null _location (struct) (`self.ProjectileClass`) true (`self.Projectile Speed`) TargetLocation _returnvalue (cast `Pawn` (`self.GetAvatarActorFromActorInfo`) :!pure true)))

(fn `GetSpawnLocation`
  (returns (Location :type "Vector Structure"))
  (bind _returnvalue (`self.GetAvatarActorFromActorInfo`))
  (bind _returnvalue_2 (`Actor.GetComponentByClass` _returnvalue "/Game/_GameplayAbilitySystem/Weapons/BP_WeaponsManager_Extended.BP_WeaponsManager_Extended_C"))
  (`/Engine/EditorBlueprintResources/StandardMacros.IsValid` _returnvalue_2
    (:`Is Valid`
      (bind _equippedweapon (`/Game/_GameplayAbilitySystem/Weapons/BP_WeaponsManager_Extended.EquippedWeapon` _returnvalue_2)
        (:`then`
          (bind _location (`/Game/_GameplayAbilitySystem/Weapons/BP_WeaponBase.GetSpawnPointLocaiton` _equippedweapon))
          (if (!= _location (0.0 0.0 0.0))
            (return _location)
            (else
              _)))
        (:`else`
          _)))
    (:`Is Not Valid`
      _))
  (return (`Actor.K2_GetActorLocation` _returnvalue)))