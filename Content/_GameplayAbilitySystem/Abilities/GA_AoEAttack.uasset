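; Gameplay ability for a two-phase, staff-based, ground-targeted AoE attack that damages pawns in a radius.
; Phase one loops a targeting montage with a camera cue while a decal target actor awaits player confirmation.
; Phase two commits, shows an indicator and plays the trigger montage, whose event fires the impact cue.
; After a short delay, an authority-only sphere trace applies SetByCaller instant damage once per actor, excluding the caster.
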(event `self.K2_ActivateAbility`
  ; AoE Attack Phase 1
  (`self.LoopTargetingAnimation`)
  (set `self.IsWaitingTargetData` true)
  (`self.K2_AddGameplayCue` (struct :`TagName` "GameplayCue._Nexus.TargetingCamera"))
  (bind (_asynctaskproxy _data) (`AbilityTask_WaitTargetData.WaitTargetData` "None" "UserConfirmed" "/Game/_GameplayAbilitySystem/Abilities/TargetingActors/GA_TargetActor_GC_decal.GA_TargetActor_GC_decal_C" "/Game/_GameplayAbilitySystem/Weapons/Decals/Decal_AOE.Decal_AOE" (`self.GetAoERadius`) 0.0 0.0 (`self.Max Range`) (struct :`Name` "NoCollision") true (`self.MakeTargetLocationInfoFromOwnerSkeletalMeshComponent` "staff_equipped_socket") (struct) null)
    (:`ValidData`
      (set `self.IsWaitingTargetData` false)
      (set `self.ConfirmedAoELocation` (`.Location` (`GameplayStatics.BreakHitResult` (`AbilitySystemBlueprintLibrary.GetHitResultFromTargetData` _data))))
      (`self.ConfirmStrike`))))

(event `LoopTargetingAnimation`
  ; AoE Attack Phase 1
  (`AbilityTask_PlayMontageAndWait.CreatePlayMontageAndWaitProxy` "None" "/Game/_GameplayAbilitySystem/Characters/Mannequins/Anims/Staff/Montage_AOE_Targeting.Montage_AOE_Targeting"
    (:`OnBlendOut`
      (if (`self.IsWaitingTargetData`)
        (`self.LoopTargetingAnimation`)))
    (:`OnInterrupted`
      (if (`self.IsWaitingTargetData`)
        (`self.K2_EndAbility`)))))

(event `ConfirmStrike`
  ; AoE Attack Phase 2
  (bind _returnvalue (`self.K2_CommitAbility`))
  (if _returnvalue
    (`self.K2_AddGameplayCueWithParams` (struct :`TagName` "GameplayCue._Nexus.AoEIndicator") (`AbilitySystemBlueprintLibrary.MakeGameplayCueParameters` 0.0 (`self.GetAoERadius`) (struct) (struct) (struct) (struct) (struct) (`self.ConfirmedAoELocation`)))
    (`AbilityTask_PlayMontageAndWait.CreatePlayMontageAndWaitProxy` "None" "/Game/_GameplayAbilitySystem/Characters/Mannequins/Anims/Staff/Montage_AOE_Trigger.Montage_AOE_Trigger"
      (:`then`
        (`AbilityTask_WaitGameplayEvent.WaitGameplayEvent` (struct :`TagName` "_Nexus.Events.Montage.Trigger") null
          (:`EventReceived`
            (`self.K2_ExecuteGameplayCueWithParams` (struct :`TagName` "GameplayCue._Nexus.AoEImpact") (`AbilitySystemBlueprintLibrary.MakeGameplayCueParameters` 0.0 0.0 (struct) (struct) (struct) (struct) (struct) (`self.ConfirmedAoELocation`) (0.0 0.0 0.0) (`self.GetAvatarActorFromActorInfo`)))
            (`KismetSystemLibrary.Delay` 0.5)
            (`self.AoEDamage`)
            (`self.K2_RemoveGameplayCue` (struct :`TagName` "GameplayCue._Nexus.AoEIndicator")))))
      (:`OnCompleted`
        (`self.K2_EndAbility` :!label _label))
      (:`OnInterrupted`
        (goto _label)))
    (else
      (`self.K2_EndAbility`))))

(event `AoEDamage`
  (bind _confirmedaoelocation (`self.ConfirmedAoELocation`))
  ; AoE Attack Phase 2
  (`self.K2_HasAuthority`
    (:`True`
      (bind _outhits (`KismetSystemLibrary.SphereTraceMultiForObjects` _confirmedaoelocation _confirmedaoelocation (`self.AoERadius`) (`|MakeArray` "ObjectTypeQuery3" :!type "EObjectTypeQuery Enum") false (`|MakeArray` (`self.GetAvatarActorFromActorInfo`)) "ForDuration"))
      (`KismetArrayLibrary.Array_Clear` (`self.HitActors`))
      (for _array_element _outhits
        (bind (_bblockinghit _binitialoverlap _time _distance _location _impactpoint _normal _impactnormal _physmat _hitactor) (`GameplayStatics.BreakHitResult` _array_element))
        (if (not (`KismetArrayLibrary.Array_Contains` (`self.HitActors`) _hitactor))
          (`KismetArrayLibrary.Array_AddUnique` (`self.HitActors`) _hitactor)
          (bind _returnvalue (`AbilitySystemBlueprintLibrary.GetAbilitySystemComponent` _hitactor))
          (`/Engine/EditorBlueprintResources/StandardMacros.IsValid` _returnvalue
            (:`Is Valid`
              (bind _returnvalue_2 (`AbilitySystemBlueprintLibrary.AssignTagSetByCallerMagnitude` (`self.MakeOutgoingGameplayEffectSpec` "/Game/_GameplayAbilitySystem/Effects/GE_DamageInstant.GE_DamageInstant_C") (struct :`TagName` "_Nexus.Data.Damage") (`self.DamageMagnitude`)))
              (`AbilitySystemComponent.BP_ApplyGameplayEffectSpecToSelf` _returnvalue _returnvalue_2))))))))

(fn `GetAoERadius`
  (returns (AoERadius :type "Float (double-precision)"))
  (return (* (`self.AoERadius`) 2.0)))